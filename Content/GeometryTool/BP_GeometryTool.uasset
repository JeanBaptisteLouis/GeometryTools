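; Generated dynamic mesh actor that procedurally builds a random, terrain-like landmass using Geometry Script.
; On mesh rebuild, it scatters randomly sized cones and appends a wide base box beneath them.
; Solidify fuses the shapes, then normals, iterative smoothing and PN tessellation soften the result before a horizontal plane cut trims it.
; A custom rebuild event forces an immediate regeneration, re-rolling the random layout.
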(event Custom|rebuild
  (DynamicMeshActor|MarkforMeshRebuild true))

(event EventBeginPlay)

(event Collision|EventActorBeginOverlap
  (params (OtherActor :type Actor%20Object%20Reference)))

(event EventTick
  (params (DeltaSeconds :type Float%20%28single-precision%29)))

(event Events|EventOnRebuildGeneratedMesh
  (params (TargetMesh :type Dynamic%20Mesh%20Object%20Reference))
  (bind _returnvalue (+ 3e+03 1e+04))
  (for _index (range 0 20)
    (Class|GeometryScriptLibraryMeshPrimitiveFunctions|AppendCone :TargetMesh TargetMesh :Transform (Math|Transform|MakeTransform (Math|Vector|MakeVector (Math|Random|RandomFloatinRange -3e+03 2e+03) (Math|Random|RandomFloatinRange -3e+03 3e+03) 0.0) "0, 0, 0" "1.000000,1.000000,1.000000") :BaseRadius (Math|Random|RandomFloatinRange 1e+03 3e+03) :TopRadius (Math|Random|RandomFloatinRange 1e+02 5e+02) :Height (Math|Random|RandomFloatinRange 6e+02 1.5e+03) :RadialSteps 32 :HeightSteps 1 :Debug 0))
  (bind _returnvalue_2 (Class|GeometryScriptLibraryMeshPrimitiveFunctions|AppendBox :TargetMesh TargetMesh :Transform (Math|Transform|MakeTransform "0.000000,0.000000,-200.000000") :DimensionX _returnvalue :DimensionY _returnvalue :DimensionZ 4e+02 :Debug 0))
  (bind _returnvalue_3 (Class|GeometryScriptLibraryMeshVoxelFunctions|ApplyMeshSolidify _returnvalue_2 (Utilities|Struct|MakeGeometryScriptSolidifyOptions (Utilities|Struct|MakeGeometryScript3DGridParameters "GridResolution" 1e+02 64) 0.5 false 0.0 64) 0))
  (bind _returnvalue_4 (Class|GeometryScriptLibraryMeshNormalsFunctions|SetPerVertexNormals _returnvalue_3 0))
  (bind _returnvalue_5 (Class|GeometryScriptLibraryMeshDeformFunctions|ApplyIterativeSmoothingtoMesh :TargetMesh _returnvalue_4 :Options (Utilities|Struct|MakeGeometryScriptIterativeMeshSmoothingOptions 6 0.2 "FullMeshSelection") :Debug 0))
  (bind _returnvalue_6 (Class|GeometryScriptLibraryMeshSubdivideFunctions|ApplyPNTessellation :TargetMesh _returnvalue_5 :TessellationLevel 2 :Debug 0))
  (Class|GeometryScriptLibraryMeshBooleanFunctions|ApplyMeshPlaneCut :TargetMesh _returnvalue_6 :CutFrame (Math|Transform|MakeTransform "0.000000,0.000000,500.000000" "0, 0, 0" "1.000000,1.000000,1.000000") :Debug 0))

(fn ConstructionScript)