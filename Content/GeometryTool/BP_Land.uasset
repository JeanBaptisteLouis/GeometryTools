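; BP_Land is a Geometry Script generated mesh actor that builds a procedural island landmass.
; On construction it draws M_DrawIsle to a render target, copies it into GreyTex via an editor-only conversion, and requests a mesh rebuild.
; The rebuild tessellates a box and repeatedly displaces a normal-angle selection with that texture at random magnitudes and UV offsets to layer islands.
; It then recomputes normals and planar-projects UVs; a plane cut is left unconnected.
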(event Custom|DrawLand
  (bind _texture_render_target (Variables|Default|GetTexture%20Render%20Target))
  (Rendering|ClearRenderTarget2D _texture_render_target)
  (Rendering|DrawMaterialtoRenderTarget _texture_render_target "/Game/GeometryTool/M_DrawIsle.M_DrawIsle")
  (EditorScripting|Rendering|ConvertRenderTargettoTexture2DEditorOnly _texture_render_target "/Game/GeometryTool/GreyTex.GreyTex")
  (DynamicMeshActor|MarkforMeshRebuild true))

(event Events|EventOnRebuildGeneratedMesh
  (params (TargetMesh :type Dynamic%20Mesh%20Object%20Reference))
  (bind _returnvalue (Class|GeometryScriptLibraryMeshPrimitiveFunctions|AppendBox :TargetMesh TargetMesh :DimensionX 1e+04 :DimensionY 1e+04 :DimensionZ 2e+03 :Debug 0))
  (bind _returnvalue_2 (Class|GeometryScriptLibraryMeshSubdivideFunctions|ApplyPNTessellation :TargetMesh _returnvalue :TessellationLevel 100 :Debug 0))
  (bind (_selection _returnvalue_3) (Class|GeometryScriptLibraryMeshSelectionFunctions|SelectMeshElementsbyNormalAngle _returnvalue_2 "0.000000,0.000000,1.000000" 1.0 "Triangles" false))
  (for _index (range 0 (Variables|Default|Getisle%20count))
    (Class|GeometryScriptLibraryMeshDeformFunctions|ApplyDisplacefromTextureMap _returnvalue_3 "/Game/GeometryTool/GreyTex.GreyTex" _selection (Utilities|Struct|MakeGeometryScriptDisplaceFromTextureOptions (Math|Random|RandomFloatinRange 3e+02 6e+02) "(X=1.000000,Y=1.000000)" (Math|Vector2D|MakeVector2D (/ (- (Math|Random|RandomFloat) 0.5) 2.0) (/ (- (Math|Random|RandomFloat) 0.5) 2.0)) 0.5 0 "FullMeshSelection") 0 0))
  (bind _returnvalue_4 (GeometryScript|Normals|RecomputeNormals TargetMesh (Utilities|Struct|MakeGeometryScriptCalculateNormalsOptions true true) false 0))
  (Class|GeometryScriptLibraryMeshUVFunctions|SetMeshUVsfromPlanarProjection :TargetMesh _returnvalue_4 :PlaneTransform (Math|Transform|MakeTransform "0, 0, 0" "0, 0, 0" "100.000000,100.000000,100.000000") :Debug 0))

(fn ConstructionScript
  (CallFunction|DrawLand))